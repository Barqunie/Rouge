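; BP_Enemy_Primary is an enemy Blueprint that displays an overhead health bar.
; On BeginPlay it creates a W_EnemyOverheadBars widget, caches the reference and assigns it to the OverhadBars widget component.
; The OnHealthChanged event forwards current and maximum health to that widget after a validity check, so the bar updates on events without polling.
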(event `self.ReceiveBeginPlay`
  (`self.SpawnOverheadBars`))

(event `self.OnHealthChanged`
  (params (CurrentHealth :type "Float (single-precision)") (MaxHealth :type "Float (single-precision)"))
  (bind _overheadbarswidgetref (`self.OverHeadBarsWidgetRef`))
  (`|ExecutionSequence`
    (:`then_0`
      (`/Engine/EditorBlueprintResources/StandardMacros.IsValid` _overheadbarswidgetref
        (:`Is Valid`
          (`/Game/Enemies/Widgets/W_EnemyOverheadBars.HealthBarPercent` _overheadbarswidgetref CurrentHealth MaxHealth))))))

(fn `SpawnOverheadBars`
  (bind _returnvalue (`|CreateWidget` "/Game/Enemies/Widgets/W_EnemyOverheadBars.W_EnemyOverheadBars_C"))
  (bind _output_get (set `self.OverHeadBarsWidgetRef` _returnvalue))
  (`WidgetComponent.SetWidget` (`self.OverhadBars`) _output_get))

(fn `UserConstructionScript`)