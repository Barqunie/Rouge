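; Gameplay ability for auto-attacking that, once activated, prints a debug string and starts an endless attack loop after a short timer.
; Each pass opens a damage window and plays the montage from AttackAnims at Counter, scaled by the attack speed multiplier.
; Completion closes the window, cycles Counter through three combo steps and immediately repeats.
; Interruption closes the window and retries the same step after a brief delay.
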(event `self.K2_ActivateAbility`
  (`KismetSystemLibrary.PrintString` "Hello")
  (`KismetSystemLibrary.K2_SetTimerDelegate` (delegate `CustomEvent`) 1.0))

(event `CustomEvent`
  (`|ExecutionSequence`
    (:`then_0`
      (`self.DamageWindowOpen`))
    (:`then_1`
      (`AbilityTask_PlayMontageAndWait.CreatePlayMontageAndWaitProxy` "None" (`|GetArrayItem` (`self.AttackAnims`) (`self.Counter`)) (`self.GetAttackSpeedMultiplier`) "None" false 1.0 0.0 true
        (:`OnCompleted`
          (`self.DamageWindowClose`)
          (if (<= (`self.Counter`) 1)
            (`/Engine/EditorBlueprintResources/StandardMacros.IncrementInt` (`self.Counter`)
              (:`  `
                _))
            (else
              (set `self.Counter` 0)))
          (`self.CustomEvent`))
        (:`OnInterrupted`
          (`self.DamageWindowClose`)
          (`KismetSystemLibrary.K2_SetTimerDelegate` (delegate `CustomEvent`) 0.4))))))