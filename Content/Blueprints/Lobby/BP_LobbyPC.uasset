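; Lobby player controller that creates the lobby UI for the local player and relays player actions to BP_LobbyGameMode.
; Setup triggers a lobby info update, R toggles ready status, and a retry event re-sends info after a short delay.
; Character selection uses a looping MultiGate to cycle through three characters via the game mode.
; Match start shows the loading screen and disables input.
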(event `self.ReceiveBeginPlay`
  (`self.SetUp`)
  (set `self.LobbyGMRef` (cast `/Game/Blueprints/Lobby/BP_LobbyGameMode` (`GameplayStatics.GetGameMode`) :!pure true)))

(event `TryAgainUpdateLobbyInfo`
  (`KismetSystemLibrary.Delay` 0.2)
  (bind _asbp_lobby_game_mode (cast `/Game/Blueprints/Lobby/BP_LobbyGameMode` (`GameplayStatics.GetGameMode`)))
  (`/Game/Blueprints/Lobby/BP_LobbyGameMode.UpdatePlayerLobbyInfo` _asbp_lobby_game_mode self))

(event `SetPlayerNameOnServer`
  (params (PlayerName :type Text))
  (bind _asbp_lobby_game_mode (cast `/Game/Blueprints/Lobby/BP_LobbyGameMode` (`GameplayStatics.GetGameMode`)))
  (`/Game/Blueprints/Lobby/BP_LobbyGameMode.UpdatePlayerLobbyInfo` _asbp_lobby_game_mode self))

(event `ToggleReadyStatusOnServer`
  (bind _playerlobbyinfopc (`self.PlayerLobbyInfoPC`))
  (setmembers `/Game/Blueprints/Lobby/S_PlayerLobbyInfo` :`StructRef` _playerlobbyinfopc :`bReady` (not (`.bReady_8_335A18B34F301B877E9453A5963A321E` (break `/Game/Blueprints/Lobby/S_PlayerLobbyInfo` _playerlobbyinfopc))))
  (bind _asbp_lobby_game_mode (cast `/Game/Blueprints/Lobby/BP_LobbyGameMode` (`GameplayStatics.GetGameMode`)))
  (`/Game/Blueprints/Lobby/BP_LobbyGameMode.UpdatePlayerLobbyInfo` _asbp_lobby_game_mode self))

(event `Key|R`
  (params (Key :type "Key Structure"))
  (:`Pressed`
    (`self.ToggleReadyStatusOnServer`)))

(event `OnStartMatch`
  (`/Game/Blueprints/Lobby/Widgets/WBP_LobbyUI.ShowLoadingScreen` (`self.LobbyUIRef`))
  (`self.DisableInput` self))

(event `SelectCharacterOnServer`
  (bind _lobbygmref (`self.LobbyGMRef`))
  (`|MultiGate` false true 1
    (:`Out 0`
      (`/Game/Blueprints/Lobby/BP_LobbyGameMode.SelectCharByIndex` (`self.LobbyGMRef`) self 0))
    (:`Out 1`
      (`/Game/Blueprints/Lobby/BP_LobbyGameMode.SelectCharByIndex` _lobbygmref self 1))
    (:`Out 2`
      (`/Game/Blueprints/Lobby/BP_LobbyGameMode.SelectCharByIndex` _lobbygmref self 2))))

(fn `SetUp`
  (bind _playerlobbyinfopc_pc (break `/Game/Blueprints/Lobby/S_PlayerLobbyInfo` (`self.PlayerLobbyInfoPC`)))
  (if (`self.IsLocalPlayerController`)
    (set `self.bShowMouseCursor` true)
    (`WidgetBlueprintLibrary.SetInputMode_GameAndUIEx` self null "DoNotLock" false)
    (bind _returnvalue (`|CreateWidget` "/Game/Blueprints/Lobby/Widgets/WBP_LobbyUI.WBP_LobbyUI_C"))
    (bind _output_get (set `self.LobbyUIRef` _returnvalue))
    (`UserWidget.AddToViewport` _output_get 0)
    (`self.SetPlayerNameOnServer` (`KismetTextLibrary.Conv_StringToText` (`AdvancedSessionsLibrary.GetPlayerName` _playerlobbyinfopc_pc)))))

(fn `UserConstructionScript`)