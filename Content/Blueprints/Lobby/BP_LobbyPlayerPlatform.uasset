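; Lobby platform actor that represents one player slot, holding that player's controller and character, with an invite-style friend list button shown while empty.
; On the server, it finds the shared BP_FriendList actor and links itself to the button widget.
; ShowFriendlist teleports that single list to this platform.
; Spawning delegates character selection to BP_LobbyGameMode and hides the button and any list parked here, while Clear destroys the character and restores the button.
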(event `self.ReceiveBeginPlay`
  (`self.SetUpServer`))

(event `SpawnCharacter`
  (params (PC :type "PlayerController Object Reference"))
  (bind _output_get (set `self.PC` PC))
  (`/Game/Blueprints/Lobby/BP_LobbyGameMode.SelectCharByIndex` (cast `/Game/Blueprints/Lobby/BP_LobbyGameMode` (`GameplayStatics.GetGameMode`) :!pure true) _output_get 0)
  (`SceneComponent.SetVisibility` (`self.OpenFriendlistButton`) false false)
  (if (== (`SceneComponent.K2_GetComponentLocation` (`self.FriendListLoc`)) (`self.K2_GetActorLocation` (`self.FriendListRef`)) :`ErrorTolerance` 1.0)
    (`/Game/Blueprints/Lobby/BP_FriendList.Show` (`self.FriendListRef`) false null)))

(event `Clear`
  (bind _currentcharacter (`self.CurrentCharacter`))
  (set `self.PC` null)
  (`/Engine/EditorBlueprintResources/StandardMacros.IsValid` _currentcharacter
    (:`Is Valid`
      (`self.K2_DestroyActor` _currentcharacter)
      (set `self.CurrentCharacter` null))
    (:`Is Not Valid`
      _))
  (`SceneComponent.SetVisibility` (`self.OpenFriendlistButton`) true false))

(fn `SetUpServer`
  (if (`KismetSystemLibrary.IsServer`)
    (bind _returnvalue (`GameplayStatics.GetActorOfClass` "/Game/Blueprints/Lobby/BP_FriendList.BP_FriendList_C"))
    (set `self.FriendListRef` _returnvalue)
    (bind _aswbp_open_friend_list_button (cast `/Game/Blueprints/Lobby/Widgets/WBP_OpenFriendListButton` (`WidgetComponent.GetWidget` (`self.OpenFriendlistButton`))))
    (set `/Game/Blueprints/Lobby/Widgets/WBP_OpenFriendListButton.LobbyPlayerPlatformRef` self _aswbp_open_friend_list_button)
    (`SceneComponent.SetVisibility` (`self.OpenFriendlistButton`) true false)))

(fn `ShowFriendlist`
  (params (bShow :type Boolean))
  (bind _returnvalue (`WidgetComponent.GetWidget` (`self.OpenFriendlistButton`)))
  (if bShow
    (`Widget.SetVisibility` _returnvalue "Collapsed")
    (`self.K2_SetActorLocation` (`self.FriendListRef`) (`SceneComponent.K2_GetComponentLocation` (`self.FriendListLoc`)) false false)
    (`/Game/Blueprints/Lobby/BP_FriendList.Show` (`self.FriendListRef`) true self)
    (else
      (`Widget.SetVisibility` _returnvalue "Visible"))))

(fn `UserConstructionScript`)